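; BP_MainPlayerController is the player controller that sets up the game's HUD and shows or hides the security camera monitor.
; On BeginPlay it creates and adds a monitor toggle widget, a hidden cameras monitor widget and a power widget to the viewport.
; It keeps a reference to the cameras monitor, and its OnMonitorOpened and OnMonitorClosed events switch that widget's visibility.
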(event EventBeginPlay
  (bind _returnvalue (UserInterface|CreateWidget "/Game/Assets/UI/MonitorToggle.MonitorToggle_C"))
  (UserInterface|Viewport|AddtoViewport _returnvalue 0)
  (bind _returnvalue_2 (UserInterface|CreateWidget "/Game/Assets/UI/WBP_CamerasMonitor.WBP_CamerasMonitor_C"))
  (bind _output_get (Variables|Default|SetREF_MonitorWidget _returnvalue_2))
  (Widget|SetVisibility _output_get "Hidden")
  (UserInterface|Viewport|AddtoViewport (Variables|Default|GetREF_MonitorWidget) 0)
  (bind _returnvalue_3 (UserInterface|CreateWidget "/Game/Assets/UI/WBP_Power.WBP_Power_C"))
  (UserInterface|Viewport|AddtoViewport _returnvalue_3 0))

(event EventOnMonitorOpened
  (Widget|SetVisibility (Variables|Default|GetREF_MonitorWidget) "Visible"))

(event EventOnMonitorClosed
  (Widget|SetVisibility (Variables|Default|GetREF_MonitorWidget) "Hidden"))

(fn ConstructionScript)