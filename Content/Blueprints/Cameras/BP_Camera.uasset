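; BP_Camera is a camera actor that rotates its root about the yaw axis by a configurable angle, starting on BeginPlay.
; It stores the root's initial world rotation and derives a target by adding RotationDegrees to the yaw.
; A timeline then drives a shortest-path rotator lerp between the two, applying the result to the root on each update.
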(event EventBeginPlay
  (bind _defaultsceneroot (Variables|Default|GetDefaultSceneRoot))
  (bind _returnvalue (Transformation|GetWorldRotation _defaultsceneroot))
  (bind (_roll _pitch _yaw) (Math|Rotator|BreakRotator _returnvalue))
  (Variables|Default|SetInitialRotation _returnvalue)
  (Variables|Default|SetTargetRotation (Math|Rotator|MakeRotator _roll _pitch (+ _yaw (Variables|Default|GetRotationDegrees))))
  (bind _newtrack_0 (Timeline|Timeline PlayFromStart)
    (:Update
      (Transformation|SetWorldRotation (Variables|Default|GetDefaultSceneRoot) (Math|Rotator|Lerp(Rotator) (Variables|Default|GetInitialRotation) (Variables|Default|GetTargetRotation) _newtrack_0 true) false false))))

(fn ConstructionScript)