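; BP_OfficeLight is an office light fixture that switches to a dim emergency-style look when the power battery drains.
; On BeginPlay it binds TurnOffLight to the PowerSubsystem's battery-drained event.
; TurnOffLight turns the spot light into a faint blue beam without color temperature, deactivates the rect light, and hides the listed static meshes.
; Nothing in the graph restores the lit state.
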(event Custom|TurnOffLight
  (bind _spotlight (Variables|Default|GetSpotLight))
  (Rendering|Components|Light|SetIntensity _spotlight 0.25)
  (Rendering|Components|Light|SetLightColor _spotlight "(R=0.000911,G=0.191202,B=0.445201,A=1.000000)" true)
  (Rendering|Lighting|SetInnerConeAngle _spotlight 42.0)
  (Class|LightComponent|SetUseTemperature _spotlight false)
  (Components|Activation|Deactivate (Variables|Default|GetRectLight))
  (for _array_element (Variables|Default|GetStaticMeshesToDisable)
    (Rendering|SetVisibility (Variables|/Script/Engine.StaticMeshActor|GetStaticMeshComponent _array_element) false false)))

(event EventBeginPlay
  (EventDispatchers|BindEventtoOnBatteryDrained (Subsystems|GetPowerSubsystem) (delegate Custom|TurnOffLight)))

(fn ConstructionScript)