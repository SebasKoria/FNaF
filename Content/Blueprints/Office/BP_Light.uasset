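; BP_Light is an interactable office light button, labelled "LIGHT" by a 3D text widget, that toggles a spotlight while unlocked.
; TurnOn and TurnOff set the spotlight's intensity, start or stop PowerDrain, and loop over LightBlockers to toggle mesh visibility and swap the button material.
; Lock, used by animatronics, forces the light off and blocks further toggling; no unlock is defined here.
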(event Custom|TurnOn
  ;[0.15 0.15 0.15 0.5] Turn On
  (if (not (Variables|Default|GetbIsOn))
    (Variables|Default|SetbIsOn true)
    (Rendering|Components|Light|SetIntensity (Variables|/Script/Engine.SpotLight|GetSpotLightComponent (Variables|Default|GetSpotLight)) 8.0)
    (Class|PowerDrainComponent|StartUsingPower (Variables|Default|GetPowerDrain))
    (for _array_element (Variables|Default|GetLightBlockers)
      (Rendering|SetVisibility (Variables|/Script/Engine.StaticMeshActor|GetStaticMeshComponent _array_element) false false)
      (Rendering|Material|SetMaterial (Variables|Default|GetButton) 0 "/Game/Assets/InteractionModels/M_LightButton_On.M_LightButton_On"))))

(event Custom|TurnOff
  ;[0.15 0.15 0.15 0.5] Turn Off
  (if (Variables|Default|GetbIsOn)
    (Variables|Default|SetbIsOn false)
    (Rendering|Components|Light|SetIntensity (Variables|/Script/Engine.SpotLight|GetSpotLightComponent (Variables|Default|GetSpotLight)) 0.0)
    (Class|PowerDrainComponent|StopUsingPower (Variables|Default|GetPowerDrain))
    (for _array_element (Variables|Default|GetLightBlockers)
      (Rendering|SetVisibility (Variables|/Script/Engine.StaticMeshActor|GetStaticMeshComponent _array_element) true false)
      (Rendering|Material|SetMaterial (Variables|Default|GetButton) 0 "/Game/Assets/InteractionModels/M_LightButton_Off.M_LightButton_Off"))))

(event EventLock
  ;[0.15 0.15 0.15 0.5] Animatronic locks the light
  (Variables|Default|SetIsLocked true)
  (CallFunction|TurnOff))

(event EventBeginPlay
  (bind _asbp_3dtext (Utilities|Casting|CastToBP_3DText (UserInterface|GetUserWidgetObject (Variables|Default|GetWidget))))
  (Default|SetText _asbp_3dtext "LIGHT"))

(event EventInteract
  ;[0.15 0.15 0.15 0.5] Toggle On/Off
  (|CallParentFunction)
  (if (not (Variables|Default|GetIsLocked))
    (if (Variables|Default|GetbIsOn)
      (CallFunction|TurnOff)
      (else
        (CallFunction|Turnon)))))

(fn ConstructionScript)