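; Interactable office door that the player toggles open and closed, drawing power while closed.
; Open and Close update the state, PowerDrain and button material, while timelines lerp the panel between its two positions.
; When an animatronic calls Lock, the door is forced open and ignores further toggling.
; BeginPlay labels the door's 3D text widget "DOOR".
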(event Custom|Open
  ;[0.15 0.15 0.15 0.5] Open the door
  (if (Variables|Default|GetbIsClosed)
    (Utilities|FlowControl|Sequence
      (:then_0
        (Variables|Default|SetbIsClosed false)
        (Class|PowerDrainComponent|StopUsingPower (Variables|Default|GetPowerDrain))
        (Rendering|Material|SetMaterial (Variables|Default|GetButton) 0 "/Game/Assets/InteractionModels/M_DoorButton_Off.M_DoorButton_Off"))
      (:then_1
        (bind _newtrack_0 (Timeline|Timeline_0 PlayFromStart)
          (:Update
            (Transformation|SetRelativeLocation (Variables|Default|GetDoor) (Math|Vector|Lerp(Vector) (Variables|Default|GetDoorClosedPosition) (Variables|Default|GetDoorOpenPosition) _newtrack_0) false true)))))))

(event Custom|Close
  ;[0.15 0.15 0.15 0.5] Close the door
  (if (not (Variables|Default|GetbIsClosed))
    (Utilities|FlowControl|Sequence
      (:then_0
        (Variables|Default|SetbIsClosed true)
        (Class|PowerDrainComponent|StartUsingPower (Variables|Default|GetPowerDrain))
        (Rendering|Material|SetMaterial (Variables|Default|GetButton) 0 "/Game/Assets/InteractionModels/M_DoorButton_On.M_DoorButton_On"))
      (:then_1
        (bind _newtrack_0 (Timeline|Timeline PlayFromStart)
          (:Update
            (Transformation|SetRelativeLocation (Variables|Default|GetDoor) (Math|Vector|Lerp(Vector) (Variables|Default|GetDoorOpenPosition) (Variables|Default|GetDoorClosedPosition) _newtrack_0) false true)))))))

(event EventLock
  ;[0.15 0.15 0.15 0.5] Animatronic locks the door
  (Variables|Default|SetisLocked true)
  (CallFunction|Open))

(event EventBeginPlay
  (bind _asbp_3dtext (Utilities|Casting|CastToBP_3DText (UserInterface|GetUserWidgetObject (Variables|Default|GetWidget))))
  (Default|SetText _asbp_3dtext "DOOR"))

(event EventInteract
  ;[0.15 0.15 0.15 0.5] Toggle Open/Close
  (|CallParentFunction)
  (if (not (Variables|Default|GetisLocked))
    (if (Variables|Default|GetbIsClosed)
      (CallFunction|Open)
      (else
        (CallFunction|Close)))))

(fn ConstructionScript)